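; Visual novel script manager that creates the HUD after a loading screen and plays the story from data tables.
; Each click skips typing or advances a script row, whose event type triggers dialog, focused image, yes/no, multiple choice, fade, background change or game over.
; Per-type tables supply lines, expressions and sounds to HUD widgets, with branching answer ranges for multiple choice.
; Yes/no answers feed points, which select the ending row.
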(event `self.ReceiveBeginPlay`
  ;[1 1 1] Main Menu Loading
  (bind _returnvalue (`|CreateWidget` "/Game/VisualNovelTemplate/Widget/WG_Loading.WG_Loading_C" (`GameplayStatics.GetPlayerController` 0)))
  (bind _output_get (set `self.Loading Screen` _returnvalue))
  (`UserWidget.AddToViewport` _output_get 0)
  (`KismetSystemLibrary.Delay` 2.0)
  (bind _returnvalue_2 (`|CreateWidget` "/Game/VisualNovelTemplate/Widget/WG_HUD.WG_HUD_C" (`GameplayStatics.GetPlayerController` 0) self))
  (set `self.HUD Ref` _returnvalue_2)
  (`Widget.RemoveFromParent` (`self.Loading Screen`))
  (`UserWidget.AddToViewport` (`self.HUD Ref`) 0)
  (`self.Get Script Now` "1")
  (`|ExecutionSequence`
    (:`then_0`
      (`self.Play Music`))
    (:`then_1`
      (`KismetSystemLibrary.Delay` 1.0)
      (`/Game/VisualNovelTemplate/Widget/WG_Dialog.Show Dialog` (`/Game/VisualNovelTemplate/Widget/WG_HUD.WG_Dialog` (`self.HUD Ref`))))))

(event `Play Msg`
  ;[1 1 1] Play  Message
  (`self.Fill Dialog`)
  (set `self.Typing` true)
  (`|ExecutionSequence`
    (:`then_0`
      ;;[1 0 0] If There is SFX Play it
      (`/Engine/EditorBlueprintResources/StandardMacros.IsValid` (`self.SFX`)
        (:`Is Valid`
          (`GameplayStatics.PlaySound2D` (`self.SFX`) 1.0 1.0 0.0 null null))))
    (:`then_1`
      (`self.Set Character Expresion`)
      (`/Game/VisualNovelTemplate/Widget/WG_Dialog.Start Msg` (`/Game/VisualNovelTemplate/Widget/WG_HUD.WG_Dialog` (`self.HUD Ref`)) (`KismetTextLibrary.Conv_StringToText` (`self.Line`)) (`self.Name`)))))

(event `Msg End`
  ;[1 1 1] End Message
  (set `self.Typing` false)
  (switch `/Game/VisualNovelTemplate/Blueprint/Enums/E_Script` (`self.Special Event`)
    (:`NewEnumerator0`
      (`KismetSystemLibrary.Delay` 1.0)
      (set `self.Is GameOver` true))
    (:`NewEnumerator1`
      (`self.Focused Event Proceed Test`))
    (:`NewEnumerator2`
      (`/Game/VisualNovelTemplate/Widget/WG_Dialog.Show Proceed` (`/Game/VisualNovelTemplate/Widget/WG_HUD.WG_Dialog` (`self.HUD Ref`)) "Visible" :!label _label)
      (`self.Enable input after first  run`))
    (:`NewEnumerator3`
      (if (`self.MC Question`)
        (set `self.MC Question` false)
        (else
          (goto _label))))
    (:`NewEnumerator4`
      (if (not (`self.YN Loop`))
        (goto _label)))
    (:`NewEnumerator5`
      (goto _label))
    (:`NewEnumerator6`
      (goto _label))))

(event `Fade in  event`
  (bind _background (`self.Background`))
  (bind _hud_ref (`self.HUD Ref`))
  ;[1 1 1] Fade in Event
  (`|ExecutionSequence`
    (:`then_0`
      (`/Engine/EditorBlueprintResources/StandardMacros.IsValid` _background
        (:`Is Valid`
          (`Image.SetBrushFromTexture` (`/Game/VisualNovelTemplate/Widget/WG_HUD.Background` (`self.HUD Ref`)) _background false))))
    (:`then_1`
      (`/Game/VisualNovelTemplate/Widget/WG_Dialog.Clear Text` (`/Game/VisualNovelTemplate/Widget/WG_HUD.WG_Dialog` _hud_ref))
      (`/Game/VisualNovelTemplate/Widget/WG_Fade.Fade In Animation Play` (`/Game/VisualNovelTemplate/Widget/WG_HUD.WG_Fade` _hud_ref)))))

(event `Hide Focused Event`
  (bind _hud_ref (`self.HUD Ref`))
  ;[1 1 1] Hide Focus
  (if (`self.Focused Active`)
    (`/Game/VisualNovelTemplate/Widget/WG_FocusedEvent.Play Pop Animation` (`/Game/VisualNovelTemplate/Widget/WG_HUD.WG_FocusedEvent` _hud_ref) "Reverse" null)
    (`Widget.SetVisibility` (`/Game/VisualNovelTemplate/Widget/WG_HUD.BackgroundBlur_107` _hud_ref) "Hidden")
    (set `self.Focused Active` false)))

(event `Focused Event`
  ;[1 1 1] Focused Event
  (`Widget.SetVisibility` (`/Game/VisualNovelTemplate/Widget/WG_HUD.BackgroundBlur_107` (`self.HUD Ref`)) "Visible")
  (`self.Play Msg`)
  (set `self.Focused Active` true)
  (set `self.Animation Playing` true)
  (`/Game/VisualNovelTemplate/Widget/WG_FocusedEvent.Play Pop Animation` (`/Game/VisualNovelTemplate/Widget/WG_HUD.WG_FocusedEvent` (`self.HUD Ref`)) "Forward" (`|GetArrayItem` (`self.FocusedEventImages`) (`self.Focused Counter`)))
  (set `self.Focused Counter` 0)
  (`/Engine/EditorBlueprintResources/StandardMacros.IncrementInt` (`self.Focused Counter`)))

(event `Change Background`
  (bind _hud_ref (`self.HUD Ref`))
  ;[1 1 1] Change Background
  (`self.Hide Focused Event`)
  (`/Game/VisualNovelTemplate/Widget/WG_Dialog.Hide Dialog` (`/Game/VisualNovelTemplate/Widget/WG_HUD.WG_Dialog` _hud_ref))
  (`Widget.SetVisibility` (`/Game/VisualNovelTemplate/Widget/WG_Character1.CharacterImage` (`/Game/VisualNovelTemplate/Widget/WG_HUD.WG_Character1` _hud_ref)) "Hidden")
  (`/Game/VisualNovelTemplate/Widget/WG_Fade.Play FadeOutIn` (`/Game/VisualNovelTemplate/Widget/WG_HUD.WG_Fade` _hud_ref))
  (`KismetSystemLibrary.Delay` 0.51)
  (`Image.SetBrushFromTexture` (`/Game/VisualNovelTemplate/Widget/WG_HUD.Background` (`self.HUD Ref`)) (`self.Background`) false))

(event `Action`
  (bind _hud_ref (`self.HUD Ref`))
  (bind _wg_dialog (`/Game/VisualNovelTemplate/Widget/WG_HUD.WG_Dialog` (`self.HUD Ref`)))
  ;[1 1 1] Action
  (set `self.CanProceed` false)
  (`/Game/VisualNovelTemplate/Widget/WG_Dialog.Clear Text` _wg_dialog)
  (`/Game/VisualNovelTemplate/Widget/WG_Dialog.Show Proceed` _wg_dialog "Hidden")
  (if (`self.MC loop`)
    (if (`self.Remaining Answers`)
      (set `self.Remaining Answers` false)
      (set `self.MC Question` true)
      (`self.MC Fill Setup Info`)
      (`/Game/VisualNovelTemplate/Widget/WG_Character1.Swap Character Position` (`/Game/VisualNovelTemplate/Widget/WG_HUD.WG_Character1` _hud_ref) "Forward" 1.0)
      (`/Game/VisualNovelTemplate/Widget/WG_MC.Play Anim` (`/Game/VisualNovelTemplate/Widget/WG_HUD.WG_MC` _hud_ref))
      (else
        (`self.Play Msg`)))
    (else
      (`self.Next Script Row`)
      (`self.Get Script Now` (`KismetStringLibrary.Conv_StringToName` (`KismetStringLibrary.Conv_IntToString` (`self.Script Counter`))))
      (`|ExecutionSequence`
        (:`then_0`
          (switch `/Game/VisualNovelTemplate/Blueprint/Enums/E_Script` (`self.Special Event`)
            (:`NewEnumerator0`
              (`self.GameOver`))
            (:`NewEnumerator1`
              (`self.Focused Event`))
            (:`NewEnumerator2`
              (`self.Play Msg`))
            (:`NewEnumerator3`
              (`self.MC Event`))
            (:`NewEnumerator4`
              (`self.Yes No`))
            (:`NewEnumerator5`
              (`self.Fade in  event`))
            (:`NewEnumerator6`
              (`self.Change Background`))))
        (:`then_1`
          ;;[1 1 1] If Music is valid then change music
          (if (not (== (`self.Script Counter`) 1))
            (`self.Play Music`)))))))

(event `Yes No`
  (bind _hud_ref (`self.HUD Ref`))
  ;[1 1 1] YN Event
  (set `self.Question Msg` true)
  (set `self.YN Loop` true)
  (set `self.YN Counter` (+ (`self.YN Counter`) 1))
  (`self.Get Row Data YN`)
  (`self.Hide Focused Event`)
  (`/Game/VisualNovelTemplate/Widget/WG_Character1.Swap Character Position` (`/Game/VisualNovelTemplate/Widget/WG_HUD.WG_Character1` _hud_ref) "Forward" 1.0)
  (`KismetSystemLibrary.Delay` 0.1)
  (`/Game/VisualNovelTemplate/Widget/WG_YN.Play Anim` (`/Game/VisualNovelTemplate/Widget/WG_HUD.WG_YN` _hud_ref)))

(event `MC Event`
  (bind _hud_ref (`self.HUD Ref`))
  ;[1 1 1] MC Event
  (set `self.MC Question` true)
  (set `self.MC loop` true)
  (`KismetArrayLibrary.Array_Clear` (`self.Selected MC Answers`))
  (`self.Hide Focused Event`)
  (`/Engine/EditorBlueprintResources/StandardMacros.IncrementInt` (`self.MC Counter`)
    (:`  `
      (`self.MC Fill Setup Info`)
      (`/Game/VisualNovelTemplate/Widget/WG_Character1.Swap Character Position` (`/Game/VisualNovelTemplate/Widget/WG_HUD.WG_Character1` _hud_ref) "Forward" 1.0)
      (`/Game/VisualNovelTemplate/Widget/WG_MC.Play Anim` (`/Game/VisualNovelTemplate/Widget/WG_HUD.WG_MC` _hud_ref)))))

(event `Key|LeftMouseButton`
  (params (Key :type "Key Structure"))
  ;[1 1 1] Inputs
  (:`Pressed`
    (if (`self.CanProceed`)
      (`self.Action`)
      (elif (`self.Typing`)
        (`/Game/VisualNovelTemplate/Widget/WG_Dialog.Break and fill msg` (`/Game/VisualNovelTemplate/Widget/WG_HUD.WG_Dialog` (`self.HUD Ref`)))
        (elif (`self.Is GameOver`)
          (bind _returnvalue (`|CreateWidget` "/Game/VisualNovelTemplate/Widget/WG_GameOver.WG_GameOver_C" (`GameplayStatics.GetPlayerController` 0)))
          (`UserWidget.AddToViewport` _returnvalue 0))))))

(fn `Add Remove Points`
  (params (Points :type Integer))
  (set `self.Points` (+ Points (`self.Points`))))

(fn `Enable input after first  run`
  (bind _returnvalue (`GameplayStatics.GetPlayerController` 0))
  (if (== (`self.Script Counter`) 1)
    (`self.EnableInput` _returnvalue)
    (set `PlayerController.bShowMouseCursor` true _returnvalue)))

(fn `Fill Dialog`
  (bind (_name _expression _startline _sfx _fiilingabc _datatablerowsa _datatablerowsb _datatablerowsc) (break `/Game/VisualNovelTemplate/Blueprint/ST_MCSetup` (`self.MC Current Row`)))
  (bind (_name_2 _expression_2 _sfx_2 _line _music _background _secondcharacter _secondcharacterexpression) (break `/Game/VisualNovelTemplate/Blueprint/ST_MCDialogSetup` (`BlueprintMapLibrary.Map_Find` (`self.MC Dialog Array`) (`self.MC Internal Row`))))
  (if (`self.YN Loop`)
    (if (`self.Question Msg`)
      (set `self.Question Msg` false)
      (else
        (bind _returnvalue (`|GetDataTableRow` (`self.DT_YN`) (`KismetStringLibrary.Conv_StringToName` (`KismetStringLibrary.Concat_StrStr` (`KismetStringLibrary.Concat_StrStr` "Q" (`KismetStringLibrary.Conv_IntToString` (`self.YN Counter`))) (`KismetMathLibrary.SelectString` "Y" "N" (`self.YN Answer`)))))
          (:`then`
            (bind (_name_3 _expression_3 _sfx_3 _line_2 _points) (break `/Game/VisualNovelTemplate/Blueprint/ST_YNDialogSetup` _returnvalue))
            (set `self.Name` _name_3)
            (set `self.Expression` _expression_3)
            (set `self.SFX` _sfx_3)
            (set `self.Line` _line_2)
            (`self.Add Remove Points` _points)
            (set `self.YN Loop` false)))))
    (elif (`self.MC loop`)
      (if (`self.MC Question`)
        _
        (elif (`.OneTime_36_02785705443D1AF5D3FCFFA3420B6CA5` (break `/Game/VisualNovelTemplate/Blueprint/ST_MCSetup` (`self.MC Current Row`)))
          (bind _returnvalue_2 (`|GetDataTableRow` (`self.DT_MCDialog`) (`KismetStringLibrary.Conv_StringToName` (`KismetStringLibrary.Conv_IntToString` (`.X` (break `IntPoint` (select `int` (`self.MC Answer`) :`0` _datatablerowsa :`1` _datatablerowsb :`2` _datatablerowsc))))))
            (:`then`
              (bind (_name_4 _expression_4 _sfx_4 _line_3 _music_2 _background_2 _secondcharacter_2 _secondcharacterexpression_2) (break `/Game/VisualNovelTemplate/Blueprint/ST_MCDialogSetup` _returnvalue_2))
              (set `self.Name` _name_4)
              (set `self.Expression` _expression_4)
              (set `self.SFX` _sfx_4)
              (set `self.Line` _line_3)
              (`self.Second Character Setup` _secondcharacterexpression_2 _secondcharacter_2)
              (set `self.MC loop` false)))
          (else
            (set `self.Name` _name_2)
            (set `self.Expression` _expression_2)
            (set `self.SFX` _sfx_2)
            (set `self.Line` _line)
            (`self.Second Character Setup` _secondcharacterexpression _secondcharacter)
            (bind _result (`/Engine/EditorBlueprintResources/StandardMacros.IncrementInt` (`self.MC Internal Row`))
              (:`  `
                (if (> _result (`self.End MC Row`))
                  (if (== (`self.MC Answer`) (`.CorrectAnswer_30_8D669FBE4CBF976BE58447A9B69E4849` (break `/Game/VisualNovelTemplate/Blueprint/ST_MCSetup` (`self.MC Current Row`))))
                    (set `self.MC loop` false)
                    (set `self.Remaining Answers` false)
                    (else
                      (set `self.Remaining Answers` true)))))))))
      (else
        (`self.Next Dialog Row`)
        (bind _returnvalue_3 (`|GetDataTableRow` (`self.DT_Dialog`) (`KismetStringLibrary.Conv_StringToName` (`KismetStringLibrary.Conv_IntToString` (`self.Dialog Counter`))))
          (:`then`
            (bind (_name_5 _expression_5 _sfx_5 _line_4) (break `/Game/VisualNovelTemplate/Blueprint/ST_DialogSetup` _returnvalue_3))
            (set `self.Name` _name_5)
            (set `self.Expression` _expression_5)
            (set `self.SFX` _sfx_5)
            (set `self.Line` _line_4)))))))

(fn `Fill MC Answer Dialog`
  (params (`MC Answer` :type Integer))
  (bind (_name _expression _startline _sfx _fiilingabc _datatablerowsa _datatablerowsb _datatablerowsc) (break `/Game/VisualNovelTemplate/Blueprint/ST_MCSetup` (`self.MC Current Row`)))
  (bind (_x _y) (break `IntPoint` (select `int` (`local.MC Answer`) :`0` _datatablerowsa :`1` _datatablerowsb :`2` _datatablerowsc)))
  (bind _output_get (set `self.MC Answer` `MC Answer`))
  (`KismetArrayLibrary.Array_Add` (`self.Selected MC Answers`) _output_get)
  (`BlueprintMapLibrary.Map_Clear` (`self.MC Dialog Array`))
  (set `self.Start MC Row` _x)
  (set `self.End MC Row` _y)
  (for _index (range (`self.Start MC Row`) (+ (`self.End MC Row`) 1))
    (bind _returnvalue (`|GetDataTableRow` (`self.DT_MCDialog`) (`KismetStringLibrary.Conv_StringToName` (`KismetStringLibrary.Conv_IntToString` _index)))
      (:`then`
        (`BlueprintMapLibrary.Map_Add` (`self.MC Dialog Array`) _index _returnvalue))))
  (set `self.MC Internal Row` (`self.Start MC Row`)))

(fn `Focused Event Proceed Test`
  (if (`KismetMathLibrary.BooleanNOR` (`self.Typing`) (`self.Animation Playing`))
    (`/Game/VisualNovelTemplate/Widget/WG_Dialog.Show Proceed` (`/Game/VisualNovelTemplate/Widget/WG_HUD.WG_Dialog` (`self.HUD Ref`)) "Visible")))

(fn `GameOver`
  (bind _points (`self.Points`))
  (bind _returnvalue (`|GetDataTableRow` (`self.DT_GameOver`) (select `bool` (>= _points 15) :`false` (select `bool` (< _points 5) :`false` "2" :`true` "3" :!type "Name") :`true` "1"))
    (:`then`
      (bind (_name _expression _sfx _line) (break `/Game/VisualNovelTemplate/Blueprint/ST_DialogSetup` _returnvalue))
      (set `self.Name` _name)
      (set `self.Expression` _expression)
      (set `self.SFX` _sfx)
      (set `self.Line` _line)
      (`self.Play Msg`))))

(fn `Get Row Data YN`
  (bind _returnvalue (`|GetDataTableRow` (`self.DT_YN`) (`KismetStringLibrary.Conv_StringToName` (`KismetStringLibrary.Concat_StrStr` "Q" (`KismetStringLibrary.Conv_IntToString` (`self.YN Counter`)))))
    (:`then`
      (bind (_name _expression _sfx _line) (break `/Game/VisualNovelTemplate/Blueprint/ST_YNDialogSetup` _returnvalue))
      (set `self.Name` _name)
      (set `self.Expression` _expression)
      (set `self.SFX` _sfx)
      (set `self.Line` _line))))

(fn `Get Script Now`
  (params (RowName :type Name))
  (bind _returnvalue (`|GetDataTableRow` (`self.DT_Script`) RowName)
    (:`then`
      (bind (_epecialevent _music _background) (break `/Game/VisualNovelTemplate/Blueprint/ST_Script` _returnvalue))
      (set `self.Special Event` _epecialevent)
      (set `self.Music` _music)
      (set `self.Background` _background))))

(fn `MC Fill Setup Info`
  (bind _wg_mc (`/Game/VisualNovelTemplate/Widget/WG_HUD.WG_MC` (`self.HUD Ref`)))
  (bind _returnvalue (`|GetDataTableRow` (`self.DT_MCSetup`) (`KismetStringLibrary.Conv_StringToName` (`KismetStringLibrary.Conv_IntToString` (`self.MC Counter`))))
    (:`then`
      (bind _output_get (set `self.MC Current Row` _returnvalue))
      (bind (_name _expression _startline _sfx _fiilingabc) (break `/Game/VisualNovelTemplate/Blueprint/ST_MCSetup` _output_get))
      (for (_array_element _array_index) _fiilingabc
        (`TextBlock.SetText` (select `int` _array_index :`0` (`/Game/VisualNovelTemplate/Widget/WG_MC.T_A` _wg_mc) :`1` (`/Game/VisualNovelTemplate/Widget/WG_MC.T_B` _wg_mc) :`2` (`/Game/VisualNovelTemplate/Widget/WG_MC.T_C` _wg_mc)) (`KismetTextLibrary.Conv_StringToText` _array_element)))
      (set `self.Name` _name)
      (set `self.Expression` _expression)
      (set `self.SFX` _sfx)
      (set `self.Line` _startline))))

(fn `Next Dialog Row`
  (set `self.Dialog Counter` (+ (`self.Dialog Counter`) 1)))

(fn `Next Script Row`
  (set `self.Script Counter` (+ (`self.Script Counter`) 1)))

(fn `Play Music`
  (bind _background_music (`self.Background Music`))
  (`/Engine/EditorBlueprintResources/StandardMacros.IsValid` (`self.Music`)
    (:`Is Valid`
      (`AudioComponent.SetSound` _background_music (`self.Music`))
      (`AudioComponent.FadeIn` _background_music 1.0 1.0 0.0 "Linear"))))

(fn `Second Character Setup`
  (params (`Second Character Expresion` :type "Texture2D Object Reference") (`Second Character` :type Boolean))
  (bind _wg_character2 (`/Game/VisualNovelTemplate/Widget/WG_HUD.WG_Character2` (`self.HUD Ref`)))
  (`/Engine/EditorBlueprintResources/StandardMacros.IsValid` `Second Character Expresion`
    (:`Is Valid`
      (`Image.SetBrushFromTexture` (`/Game/VisualNovelTemplate/Widget/WG_Character2.CharacterImage` _wg_character2) `Second Character Expresion` true))
    (:`Is Not Valid`
      _))
  (if `Second Character`
    (if (not (`/Game/VisualNovelTemplate/Widget/WG_Character2.Poped` _wg_character2))
      (`/Game/VisualNovelTemplate/Widget/WG_Character2.Character Pop` _wg_character2 "Forward" 1.0))
    (elif (`/Game/VisualNovelTemplate/Widget/WG_Character2.Poped` _wg_character2)
      (`/Game/VisualNovelTemplate/Widget/WG_Character2.Character Pop` _wg_character2 "Reverse" 1.0))))

(fn `Set Character Expresion`
  (bind _expression (`self.Expression`))
  (bind _characterimage (`/Game/VisualNovelTemplate/Widget/WG_Character1.CharacterImage` (`/Game/VisualNovelTemplate/Widget/WG_HUD.WG_Character1` (`self.HUD Ref`))))
  (`/Engine/EditorBlueprintResources/StandardMacros.IsValid` _expression
    (:`Is Valid`
      (`Image.SetBrushFromTexture` _characterimage _expression true)
      (`Widget.SetVisibility` _characterimage "Visible"))))

(fn `UserConstructionScript`)