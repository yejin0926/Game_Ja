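; Anaconda wildlife AI that idles, roams around its spawn point, rests, flees and revives after death.
; Delay-driven event loops drain and regain energy and health, feeding a randomized decision cycle gated by state flags.
; AI Perception triggers a reaction animation and flight, while hits reduce health, causing flight or death followed by a timed revival.
; Movement uses AIMoveTo to random reachable points, and actions set an enum on the Anim Blueprint.
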(event `self.ReceiveBeginPlay`
  ;[1 1 1] Start
  (`self.Decide Action` false)
  (`self.Drain Energy`)
  (`KismetSystemLibrary.Delay` 1.0)
  (set `self.HomeLocation` (`self.K2_GetActorLocation`)))

(event `Decide Action`
  (params (`Skip Delay?` :type Boolean))
  (bind _wait_ (`self.Wait?`))
  (bind _dead_ (`self.Dead?`))
  ;[1 1 1] Decide
  (if `Skip Delay?`
    (if _dead_
      _
      (elif _wait_
        _
        (elif (not (`self.Resting?`))
          (if (`self.Tired?`) :!label _label
            (`KismetSystemLibrary.Delay` 1.0 :!label _label_2)
            (`self.Rest`)
            (elif (>= (`self.Decide Logic`) 4)
              (set `self.Tired?` true)
              (goto _label_2)
              (else
                (`KismetSystemLibrary.Delay` 1.0)
                (`self.Roam`)
                (`self.Drain Energy`))))
          (`self.Random Logic`))))
    (elif _dead_
      _
      (elif _wait_
        _
        (elif (not (`self.Resting?`))
          (if (< (`self.Health`) (`self.Max Heath`))
            (`self.Regain Health`))
          (set `self.Decide Logic` (`KismetMathLibrary.RandomIntegerInRange` 0 5))
          (set `self.Idle Random Count` 0)
          (set `self.Idle Random Time` (`KismetMathLibrary.RandomIntegerInRange` (`self.Idle Time Min`) (`self.Idle Time Max`)))
          (bind _output_get (set `self.Idle Random Count` (+ (`self.Idle Random Count`) 1) :!label _label_3))
          (if (== _output_get (`self.Idle Random Time`))
            (goto _label)
            (elif (`self.Tired?`)
              (goto _label_2)
              (elif (`self.Run?`)
                _
                (elif (not (`self.Dead?`))
                  (`KismetSystemLibrary.Delay` 1.0)
                  (goto _label_3))))))))))

(event `Random Logic`
  ;[1 1 1] Logic
  (`KismetSystemLibrary.Delay` 2.0)
  (set `self.Logic?` true)
  (set `self.Decide Logic Time` 0)
  (if (<= (`self.Decide Logic`) 2)
    ;[1 1 1] Roaming Visual
    (`KismetSystemLibrary.Delay` 1.0 :!label _label_4)
    (if (`self.Wait?`)
      (goto _label_4)
      (else
        _))
    (else
      (if (>= (`self.Decide Logic`) 4) :!label _label_5
        (set `self.Decide Logic Random` (`KismetMathLibrary.RandomIntegerInRange` (`self.Resting Time Min`) (`self.Resting Time Max`)))
        (set `self.Decide Logic Time` 0)
        (`KismetSystemLibrary.Delay` 1.0 :!label _label_6)
        (bind _output_get (set `self.Decide Logic Time` (+ (`self.Decide Logic Time`) 1)))
        (if (== _output_get (`self.Decide Logic Random`))
          (set `self.Decide Logic` (`KismetMathLibrary.RandomIntegerInRange` 0 5))
          (goto _label_5)
          (elif (`self.Resting?`)
            (if (`self.Run?`)
              _
              (else
                (goto _label_6))))))))
  (set `self.Logic?` false))

(event `Drain Energy`
  ;[1 1 1] Drain Energy
  (if (`self.Resting?`)
    _
    (elif (`self.Dead?`)
      _
      (elif (`self.Run?`)
        (bind _output_get (set `self.Energy` (`KismetMathLibrary.Clamp` (- (`self.Energy`) (`self.Run Energy Drain`)) 0 (`self.Max Energy`))))
        (if (== _output_get 0)
          (`KismetSystemLibrary.Delay` 1.0)
          (set `self.Tired?` true :!label _label_7)
          (set `self.Decide Logic` 4)
          (`self.Decide Action` true)
          (else
            (`KismetSystemLibrary.Delay` 1.0 :!label _label_8)
            (`self.Drain Energy`)))
        (else
          (bind _output_get_2 (set `self.Energy` (`KismetMathLibrary.Clamp` (- (`self.Energy`) (`self.Energy Drain`)) 0 (`self.Max Energy`))))
          (if (<= _output_get_2 1)
            (`KismetSystemLibrary.Delay` 1.0)
            (goto _label_7)
            (else
              (goto _label_8))))))))

(event `Regain Energy`
  ;[1 1 1] Regain Energy
  (if (`self.Resting?`)
    (if (`self.Dead?`)
      _
      (elif (not (`self.Run?`))
        (bind _output_get (set `self.Energy` (`KismetMathLibrary.Clamp` (+ (`self.Energy`) (`self.Energy Gain`)) 0 (`self.Max Energy`))))
        (if (== _output_get (`self.Max Energy`))
          (set `self.Tired?` false)
          (set `self.Decide Logic` 2)
          (`self.Decide Action` false)
          (else
            (`KismetSystemLibrary.Delay` 1.0)
            (`self.Regain Energy`)))))))

(event `Rest`
  ;[1 1 1] Rest
  (if (`self.Dead?`)
    _
    (elif (`self.Resting?`)
      _
      (elif (`self.Tired?`)
        (if (not (`self.Run?`))
          (`MovementComponent.StopMovementImmediately` (`self.CharacterMovement`))
          (set `self.Resting?` true)
          (`self.Regain Energy`)
          (bind _asanaconda_anim_blueprint (cast `/Game/Medhue_Anaconda/Blueprints/Anaconda_AnimBlueprint` (`SkeletalMeshComponent.GetAnimInstance` (`self.Mesh`))))
          (set `/Game/Medhue_Anaconda/Blueprints/Anaconda_AnimBlueprint.Anaconda_Actions` "NewEnumerator2" _asanaconda_anim_blueprint)
          (`KismetSystemLibrary.Delay` 5.0)
          (set `/Game/Medhue_Anaconda/Blueprints/Anaconda_AnimBlueprint.Anaconda_Actions` "NewEnumerator3" _asanaconda_anim_blueprint)
          (`KismetSystemLibrary.Delay` 1.0 :!label _label_9)
          (if (`self.Dead?`)
            _
            (elif (not (`self.Run?`))
              (if (>= (`self.Decide Logic`) 3)
                (if (`self.Tired?`)
                  (goto _label_9)
                  (else
                    _)))
              (set `self.Tired?` false)
              (set `self.Resting?` false)
              (set `/Game/Medhue_Anaconda/Blueprints/Anaconda_AnimBlueprint.Anaconda_Actions` "NewEnumerator4" _asanaconda_anim_blueprint)
              (`KismetSystemLibrary.Delay` 5.7)
              (set `/Game/Medhue_Anaconda/Blueprints/Anaconda_AnimBlueprint.Anaconda_Actions` "NewEnumerator0" _asanaconda_anim_blueprint)
              (`self.Decide Action` true)
              (`self.Drain Energy`))))
        (else
          (`KismetSystemLibrary.Delay` 5.0)
          (`self.Decide Action` true))))))

(event `Roam`
  ;[1 1 1] Roam
  (if (`self.Run?`)
    _
    (elif (not (`self.Dead?`))
      (if (not (`self.Tired?`))
        (set `CharacterMovementComponent.MaxWalkSpeed` (`self.Walk Speed`) (`self.CharacterMovement`))
        (bind _asanaconda_anim_blueprint (cast `/Game/Medhue_Anaconda/Blueprints/Anaconda_AnimBlueprint` (`SkeletalMeshComponent.GetAnimInstance` (`self.Mesh`))))
        (set `/Game/Medhue_Anaconda/Blueprints/Anaconda_AnimBlueprint.Anaconda_Actions` "NewEnumerator0" _asanaconda_anim_blueprint)
        (set `self.Wait?` true)
        (`|AIMoveTo` self (`NavigationSystemV1.K2_GetRandomReachablePointInRadius` (`self.HomeLocation`) (`self.Walk Radius`) null null) null
          (:`OnSuccess`
            _)
          (:`OnFail`
            _))
        (set `self.Wait?` false)
        (`KismetSystemLibrary.Delay` 1.0))
      (`self.Decide Action` false))))

(event `Damage`
  (bind _charactermovement (`self.CharacterMovement`))
  (bind _returnvalue (`SkeletalMeshComponent.GetAnimInstance` (`self.Mesh`)))
  ;[1 1 1] Damage
  (if (not (`self.Dead?`))
    (bind _output_get (set `self.Health` (`KismetMathLibrary.Clamp` (- (`self.Health`) (`self.Health Drain`)) 0 (`self.Max Heath`))))
    (if (== _output_get 0)
      (`MovementComponent.StopMovementImmediately` _charactermovement)
      (set `self.Dead?` true)
      (bind _asanaconda_anim_blueprint (cast `/Game/Medhue_Anaconda/Blueprints/Anaconda_AnimBlueprint` _returnvalue))
      (set `/Game/Medhue_Anaconda/Blueprints/Anaconda_AnimBlueprint.Anaconda_Actions` "NewEnumerator6" _asanaconda_anim_blueprint)
      (`KismetSystemLibrary.Delay` 1.9)
      (set `/Game/Medhue_Anaconda/Blueprints/Anaconda_AnimBlueprint.Anaconda_Actions` "NewEnumerator8" _asanaconda_anim_blueprint)
      (set `self.Hit?` false)
      (set `self.Run?` true)
      (set `self.Wait?` false)
      (set `self.Resting?` false)
      (set `self.Tired?` false)
      (`KismetSystemLibrary.Delay` (`KismetMathLibrary.Conv_IntToDouble` (`KismetMathLibrary.RandomIntegerInRange` (`self.Dead Time Min`) (`self.Dead Time Max`))))
      (`self.Alive`)
      (else
        (`MovementComponent.StopMovementImmediately` _charactermovement)
        (bind _asanaconda_anim_blueprint_2 (cast `/Game/Medhue_Anaconda/Blueprints/Anaconda_AnimBlueprint` _returnvalue))
        (set `/Game/Medhue_Anaconda/Blueprints/Anaconda_AnimBlueprint.Anaconda_Actions` "NewEnumerator6" _asanaconda_anim_blueprint_2)
        (set `self.Hit?` false)
        (set `self.Run?` true)
        (set `self.Wait?` false)
        (set `self.Resting?` false)
        (set `self.Tired?` false)
        (`self.Run Away`)))))

(event `Run Away`
  ;[1 1 1] Run Away
  (if (not (`self.Dead?`))
    (set `CharacterMovementComponent.MaxWalkSpeed` (`self.Run Speed`) (`self.CharacterMovement`))
    (bind _asanaconda_anim_blueprint (cast `/Game/Medhue_Anaconda/Blueprints/Anaconda_AnimBlueprint` (`SkeletalMeshComponent.GetAnimInstance` (`self.Mesh`))))
    (set `/Game/Medhue_Anaconda/Blueprints/Anaconda_AnimBlueprint.Anaconda_Actions` "NewEnumerator0" _asanaconda_anim_blueprint)
    (set `self.Wait?` true)
    (`|AIMoveTo` self (`NavigationSystemV1.K2_GetRandomReachablePointInRadius` (`self.K2_GetActorLocation`) (`KismetMathLibrary.RandomFloatInRange` (`self.Run Radius Min`) (`self.Run Radius Max`)) null null) null
      (:`OnSuccess`
        _)
      (:`OnFail`
        _))
    (set `self.Run?` false)
    (set `self.Wait?` false)
    (`KismetSystemLibrary.Delay` 0.5)
    (`self.Decide Action` false)))

(event `self.AIPerception.OnTargetPerceptionUpdated`
  (params (Actor :type "Actor Object Reference") (Stimulus :type "AIStimulus Structure"))
  (bind _dead_ (`self.Dead?`))
  (bind _returnvalue (`SkeletalMeshComponent.GetAnimInstance` (`self.Mesh`)))
  ;[1 1 1] Detect
  (if (`self.SightOff?`)
    _
    (elif (`self.Seen?`)
      _
      (elif (`self.Dead?`)
        _
        (elif (not (`self.Run?`))
          (set `self.Seen?` true)
          (`MovementComponent.StopMovementImmediately` (`self.CharacterMovement`))
          (if (`self.Resting?`)
            (bind _asanaconda_anim_blueprint (cast `/Game/Medhue_Anaconda/Blueprints/Anaconda_AnimBlueprint` _returnvalue))
            (set `/Game/Medhue_Anaconda/Blueprints/Anaconda_AnimBlueprint.Anaconda_Actions` "NewEnumerator9" _asanaconda_anim_blueprint)
            (`KismetSystemLibrary.Delay` 1.6)
            (if (not _dead_)
              (set `/Game/Medhue_Anaconda/Blueprints/Anaconda_AnimBlueprint.Anaconda_Actions` "NewEnumerator5" _asanaconda_anim_blueprint)
              (`KismetSystemLibrary.Delay` 1.4)
              (if (not _dead_) :!label _label_10
                (set `self.Run?` true)
                (set `self.Resting?` false)
                (set `self.Wait?` false)
                (set `self.Tired?` false)
                (`self.Run Away`)))
            (else
              (bind _asanaconda_anim_blueprint_2 (cast `/Game/Medhue_Anaconda/Blueprints/Anaconda_AnimBlueprint` _returnvalue)
                (:`then`
                  (set `/Game/Medhue_Anaconda/Blueprints/Anaconda_AnimBlueprint.Anaconda_Actions` "NewEnumerator5" _asanaconda_anim_blueprint_2))
                (:`CastFailed`
                  _))
              (`KismetSystemLibrary.Delay` 1.2)
              (goto _label_10)))
          (`KismetSystemLibrary.Delay` 5.0)
          (set `self.Seen?` false))))))

(event `Alive`
  ;[1 1 1] Revive
  (set `self.Health` (`self.Max Heath`))
  (set `self.Energy` (`self.Max Energy`))
  (set `self.Dead?` false)
  (set `self.Hit?` false)
  (set `self.Run?` false)
  (set `self.Wait?` false)
  (set `self.Resting?` false)
  (set `self.Tired?` false)
  (bind _asanaconda_anim_blueprint (cast `/Game/Medhue_Anaconda/Blueprints/Anaconda_AnimBlueprint` (`SkeletalMeshComponent.GetAnimInstance` (`self.Mesh`))))
  (set `/Game/Medhue_Anaconda/Blueprints/Anaconda_AnimBlueprint.Anaconda_Actions` "NewEnumerator0" _asanaconda_anim_blueprint)
  (`self.Decide Action` false))

(event `self.ReceiveHit`
  (params (MyComp :type "PrimitiveComponent Object Reference") (Other :type "Actor Object Reference") (OtherComp :type "PrimitiveComponent Object Reference") (bSelfMoved :type Boolean) (HitLocation :type "Vector Structure") (HitNormal :type "Vector Structure") (NormalImpulse :type "Vector Structure") (Hit :type "HitResult Structure (by ref)"))
  ;[1 1 1] Hit Check
  (if (`self.DeathOff?`)
    (if (not (`self.Dead?`))
      (set `self.Resting?` false)
      (set `self.Hit?` true)
      (set `self.Wait?` false)
      (set `self.Tired?` false)
      (`self.Damage`)
      (`KismetSystemLibrary.Delay` 5.0)
      (set `self.Hit?` false))))

(event `Regain Health`
  ;[1 1 1] Regain Health
  (if (not (`self.Dead?`))
    (bind _output_get (set `self.Health` (`KismetMathLibrary.Clamp` (+ (`self.Health`) 1) 0 (`self.Max Heath`))))
    (if (not (== _output_get (`self.Max Heath`)))
      (`KismetSystemLibrary.Delay` 2.0)
      (`self.Regain Health`))))

(fn `UserConstructionScript`)